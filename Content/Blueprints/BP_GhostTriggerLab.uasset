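; BP_GhostTriggerLab is a one-shot scare trigger that sends a ghost actor moving when the player pawn overlaps it.
; The first overlap plays a sinister piano chord at the ghost and starts the run, then hides the ghost after a three-second delay.
; While running, Tick slides the ghost along Direction without sweeping, scaling Speed by delta time and 100.
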(event Collision|EventActorBeginOverlap
  (params (OtherActor :type Actor%20Object%20Reference))
  (if (== OtherActor (Game|Player|GetPlayerPawn 0))
    (if (not (Variables|Default|GetonlyOnce))
      (Variables|Default|SetonlyOnce true)
      (Variables|Default|SetisRunning true)
      (Audio|PlaySoundatLocation "/Game/Audio/Sounds/Ghost/Sinister_Piano_Chord.Sinister_Piano_Chord" (Transformation|GetActorLocation (Variables|Default|GetGhost)))
      (Utilities|FlowControl|Delay 3.0)
      (Variables|Default|SetisRunning false)
      (Rendering|SetActorHiddenInGame (Variables|Default|GetGhost) true))))

(event EventTick
  (params (DeltaSeconds :type Float%20%28single-precision%29))
  (bind _ghost (Variables|Default|GetGhost))
  (if (Variables|Default|GetisRunning)
    (Transformation|SetActorLocation _ghost (+ (Transformation|GetActorLocation _ghost) (* (Variables|Default|Getdirection) (* (* DeltaSeconds (Variables|Default|Getspeed)) 1e+02))) false false)))

(fn ConstructionScript)
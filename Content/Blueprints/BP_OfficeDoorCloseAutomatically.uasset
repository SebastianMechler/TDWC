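; A one-shot trigger actor that shuts an office door behind the player.
; When the player pawn first overlaps it, it closes the referenced OfficeDoor if open by calling Interact, then locks it and shuts down its gas trap.
; An OnlyOnce flag prevents it from firing again.
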(event EventBeginPlay)

(event Collision|EventActorBeginOverlap
  (params (OtherActor :type Actor%20Object%20Reference))
  (bind _returnvalue (Game|Player|GetPlayerPawn 0))
  (bind _officedoor (Variables|Default|GetOfficeDoor))
  (if (== OtherActor _returnvalue)
    (if (not (Variables|Default|GetonlyOnce))
      (bind _returnvalue_2 (Class|InteractableDoor|GetOpenState _officedoor))
      (if _returnvalue_2
        (Class|InteractableDoor|Interact _officedoor _returnvalue))
      (Class|InteractableDoor|SetLockState _officedoor true)
      (Class|InteractableDoor|ShutdownGasTrap _officedoor)
      (Variables|Default|SetonlyOnce true))))

(fn ConstructionScript)